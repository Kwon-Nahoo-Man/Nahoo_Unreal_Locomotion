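; Traversable box actor for the locomotion system that supplies front and back ledge data to traversal checks.
; The construction script registers four edge splines and maps each to its opposite.
; GetLedgeTransform picks the spline nearest the actor, using an up-vector offset, then clamps the hit point within it by minimum ledge width.
; The opposite spline supplies the back ledge, with spline up vectors serving as ledge normals.
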(fn `FindClosestLedge`
  (params (ActorLocation :type "Vector Structure"))
  (returns (ReturnValue :type "SplineComponent Object Reference"))
  (locals (ClosestDistance :type "Float (double-precision)") (ClosestIndex :type Integer))
  (bind _actorlocation (`local.ActorLocation`))
  (if (`KismetArrayLibrary.Array_IsNotEmpty` (`self.m-SplineArray`))
    (for (_array_element _array_index) (`self.m-SplineArray`)
      (bind _returnvalue (`KismetMathLibrary.Vector_Distance` (+ (`SplineComponent.FindLocationClosestToWorldLocation` _array_element _actorlocation "World") (* (`SplineComponent.FindUpVectorClosestToWorldLocation` _array_element _actorlocation "World") 10.0)) (`local.ActorLocation`)))
      (if (or (< _returnvalue (`local.ClosestDistance`)) (== _array_index 0))
        (set `local.ClosestDistance` _returnvalue)
        (set `local.ClosestIndex` _array_index)))
    (return (`|GetArrayItem` (`self.m-SplineArray`) (`local.ClosestIndex`)))
    (else
      (return null))))

(fn `GetLedgeTransform`
  (params (HitLocation :type "Vector Structure") (ActorLocation :type "Vector Structure") (OutTraversalCheckResult :type "/Game/Nahoo_Locomotion_System/Data/Struct/S-TraversalCheckResult Structure (by ref)"))
  (locals (ClosestLedge :type "SplineComponent Object Reference") (OppositeLedge :type "SplineComponent Object Reference"))
  (bind (_value _returnvalue) (`BlueprintMapLibrary.Map_Find` (`self.m-OppositeLedges`) (`local.ClosestLedge`)))
  (bind (_returnvalue_location _returnvalue_rotation) (`KismetMathLibrary.BreakTransform` (`SplineComponent.FindTransformClosestToWorldLocation` (`local.OppositeLedge`) (`.FrontLedgeLocation_21_65FDBC994801611C94E82BB6FD32AB14` (break `/Game/Nahoo_Locomotion_System/Data/Struct/S-TraversalCheckResult` OutTraversalCheckResult)) "World" false)))
  (bind _returnvalue_2 (/ (`self.m-MinLedgeWidth`) 2.0))
  (bind (_returnvalue_location_2 _returnvalue_rotation_2) (`KismetMathLibrary.BreakTransform` (`SplineComponent.GetTransformAtDistanceAlongSpline` (`local.ClosestLedge`) (`KismetMathLibrary.FClamp` (`SplineComponent.GetDistanceAlongSplineAtLocation` (`local.ClosestLedge`) (`SplineComponent.FindLocationClosestToWorldLocation` (`local.ClosestLedge`) (`local.HitLocation`) "Local") "Local") _returnvalue_2 (- (`SplineComponent.GetSplineLength` (`local.ClosestLedge`)) _returnvalue_2)) "World" false)))
  (`|ExecutionSequence`
    (:`then_0`
      (bind _returnvalue_3 (`self.FindClosestLedge` (`local.ActorLocation`)))
      (`/Engine/EditorBlueprintResources/StandardMacros.IsValid` _returnvalue_3
        (:`Is Valid`
          (set `local.ClosestLedge` _returnvalue_3)
          (if (>= (`SplineComponent.GetSplineLength` (`local.ClosestLedge`)) (`self.m-MinLedgeWidth`))
            (setmembers `/Game/Nahoo_Locomotion_System/Data/Struct/S-TraversalCheckResult` :`StructRef` OutTraversalCheckResult :`HasFrontLedge` true :`FrontLedgeLocation` _returnvalue_location_2 :`FrontLedgeNormal` (`KismetMathLibrary.GetUpVector` _returnvalue_rotation_2))
            (else
              (setmembers `/Game/Nahoo_Locomotion_System/Data/Struct/S-TraversalCheckResult` :`StructRef` OutTraversalCheckResult :`HasFrontLedge` false)
              (return))))
        (:`Is Not Valid`
          (setmembers `/Game/Nahoo_Locomotion_System/Data/Struct/S-TraversalCheckResult` :`StructRef` OutTraversalCheckResult :`HasFrontLedge` false)
          (return))))
    (:`then_1`
      (if _returnvalue
        (set `local.OppositeLedge` _value)
        (setmembers `/Game/Nahoo_Locomotion_System/Data/Struct/S-TraversalCheckResult` :`StructRef` OutTraversalCheckResult :`HasBackLedge` true :`BackLedgeLocation` _returnvalue_location :`BackLedgeNormal` (`KismetMathLibrary.GetUpVector` _returnvalue_rotation))
        (else
          (setmembers `/Game/Nahoo_Locomotion_System/Data/Struct/S-TraversalCheckResult` :`StructRef` OutTraversalCheckResult :`HasBackLedge` false)
          (return))))))

(fn `UserConstructionScript`
  (set `self.m-SplineArray` (`|MakeArray` (`self.Spline1`) (`self.Spline2`) (`self.Spline3`) (`self.Spline4`)))
  (set `self.m-OppositeLedges` (`|MakeMap` (`self.Spline1`) (`self.Spline2`) (`self.Spline2`) (`self.Spline1`) (`self.Spline3`) (`self.Spline4`) (`self.Spline4`) (`self.Spline3`))))