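; Base character of the Nahoo locomotion system, turning Enhanced Input into walk, run, sprint, strafe, aim, crouch and jump.
; A prerequisite component ticks rotation and movement updates before CharacterMovement.
; Strafe or aim switches to controller-facing rotation; gait and velocity drive acceleration and friction, pending input sets braking, and a direction curve blends directional max speeds.
; Landing velocity and a brief just-landed flag are recorded.
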(event `self.OnLanded`
  (params (Hit :type "HitResult Structure (by ref)"))
  (set `self.m-landVelocity` (`MovementComponent.Velocity` (`self.CharacterMovement`)))
  (set `self.m-justLanded` true)
  (`KismetSystemLibrary.RetriggerableDelay` 0.3)
  (set `self.m-justLanded` false))

(event `self.ReceiveBeginPlay`
  (`ActorComponent.AddTickPrerequisiteComponent` (`self.CharacterMovement`) (`self.comp-PreCMC`)))

(event `self.OnWalkingOffLedge`
  (params (PreviousFloorImpactNormal :type "Vector Structure (by ref)") (PreviousFloorContactNormal :type "Vector Structure (by ref)") (PreviousLocation :type "Vector Structure (by ref)") (TimeDelta :type "Float (single-precision)"))
  (`self.UnCrouch`))

(event `PreCMCTick`
  ;[0.3229 0.5208 0.3831 0.5] Update before the Character Component update
  (`self.UpdateRotation`)
  (`self.UpdateMovement`))

(event `EnhancedInput|/Game/Nahoo_Locomotion_System/Input/Actions/IA-Walk`
  (params (ActionValue :type Boolean) (ElapsedSeconds :type "Float (double-precision)") (TriggeredSeconds :type "Float (double-precision)") (InputAction :type "InputAction Object Reference" :default "/Game/Nahoo_Locomotion_System/Input/Actions/IA-Walk.IA-Walk"))
  (:`Started`
    (`self.Nahoo_WalkToggle`)))

(event `EnhancedInput|/Game/Nahoo_Locomotion_System/Input/Actions/IA-Move`
  (params (ActionValue :type "Vector2D Structure") (ElapsedSeconds :type "Float (double-precision)") (TriggeredSeconds :type "Float (double-precision)") (InputAction :type "InputAction Object Reference" :default "/Game/Nahoo_Locomotion_System/Input/Actions/IA-Move.IA-Move"))
  (:`Triggered`
    (`self.Nahoo_Move` ActionValue_X ActionValue_Y)))

(event `EnhancedInput|/Game/Nahoo_Locomotion_System/Input/Actions/IA-Sprint`
  (params (ActionValue :type Boolean) (ElapsedSeconds :type "Float (double-precision)") (TriggeredSeconds :type "Float (double-precision)") (InputAction :type "InputAction Object Reference" :default "/Game/Nahoo_Locomotion_System/Input/Actions/IA-Sprint.IA-Sprint"))
  (:`Triggered`
    (setmembers `/Game/Nahoo_Locomotion_System/Data/Struct/S-InputState` :`StructRef` (`self.m-inputState`) :`Want to Walk` false :`Want to Sprint` ActionValue :!label _label))
  (:`Completed`
    (goto _label)))

(event `EnhancedInput|/Game/Nahoo_Locomotion_System/Input/Actions/IA-Look`
  (params (ActionValue :type "Vector2D Structure") (ElapsedSeconds :type "Float (double-precision)") (TriggeredSeconds :type "Float (double-precision)") (InputAction :type "InputAction Object Reference" :default "/Game/Nahoo_Locomotion_System/Input/Actions/IA-Look.IA-Look"))
  (:`Triggered`
    (`self.Nahoo_Look` ActionValue_Y ActionValue_X)))

(event `EnhancedInput|/Game/Nahoo_Locomotion_System/Input/Actions/IA-Jump`
  (params (ActionValue :type Boolean) (ElapsedSeconds :type "Float (double-precision)") (TriggeredSeconds :type "Float (double-precision)") (InputAction :type "InputAction Object Reference" :default "/Game/Nahoo_Locomotion_System/Input/Actions/IA-Jump.IA-Jump"))
  (:`Started`
    (`self.Nahoo_Jump` ActionValue :!label _label_2))
  (:`Completed`
    (goto _label_2)))

(event `EnhancedInput|/Game/Nahoo_Locomotion_System/Input/Actions/IA-Strafe`
  (params (ActionValue :type Boolean) (ElapsedSeconds :type "Float (double-precision)") (TriggeredSeconds :type "Float (double-precision)") (InputAction :type "InputAction Object Reference" :default "/Game/Nahoo_Locomotion_System/Input/Actions/IA-Strafe.IA-Strafe"))
  (:`Started`
    (setmembers `/Game/Nahoo_Locomotion_System/Data/Struct/S-InputState` :`StructRef` (`self.m-inputState`) :`Want to Strafe` (not (`.WanttoStrafe_4_485767C946B920090F31B3BADF768C4E` (break `/Game/Nahoo_Locomotion_System/Data/Struct/S-InputState` (`self.m-inputState`)))))))

(event `EnhancedInput|/Game/Nahoo_Locomotion_System/Input/Actions/IA-Crouch`
  (params (ActionValue :type Boolean) (ElapsedSeconds :type "Float (double-precision)") (TriggeredSeconds :type "Float (double-precision)") (InputAction :type "InputAction Object Reference" :default "/Game/Nahoo_Locomotion_System/Input/Actions/IA-Crouch.IA-Crouch"))
  (:`Started`
    (`self.Nahoo_Crouch`)))

(event `EnhancedInput|/Game/Nahoo_Locomotion_System/Input/Actions/IA-Aim`
  (params (ActionValue :type Boolean) (ElapsedSeconds :type "Float (double-precision)") (TriggeredSeconds :type "Float (double-precision)") (InputAction :type "InputAction Object Reference" :default "/Game/Nahoo_Locomotion_System/Input/Actions/IA-Aim.IA-Aim"))
  (:`Triggered`
    (setmembers `/Game/Nahoo_Locomotion_System/Data/Struct/S-InputState` :`StructRef` (`self.m-inputState`) :`Want to Aim` ActionValue :!label _label_3))
  (:`Completed`
    (goto _label_3)))

(fn `CalculateBrakingDeceleration`
  (returns (`Return Value` :type "Float (double-precision)"))
  (return (select `bool` (!= (`PawnMovementComponent.GetPendingInputVector` (`self.CharacterMovement`)) (0.0 0.0 0.0) :`ErrorTolerance` 0.01) :`false` 2000.0 :`true` 500.0)))

(fn `CalculateCrouchMaxSpeed`
  (returns (`Return Value` :type "Float (double-precision)"))
  (locals (StrafeMapValue :type "Float (double-precision)"))
  (bind _y (.y (100.0 50.0 30.0)))
  (set `local.StrafeMapValue` (select `bool` (`CharacterMovementComponent.bUseControllerDesiredRotation` (`self.CharacterMovement`)) :`true` (`CurveFloat.GetFloatValue` (`self.m-strafeMap`) (`KismetMathLibrary.Abs` (`KismetAnimationLibrary.CalculateDirection` (`MovementComponent.Velocity` (`self.CharacterMovement`)) (`self.K2_GetActorRotation`))))))
  (return (`KismetMathLibrary.SelectFloat` (`KismetMathLibrary.MapRangeClamped` (`local.StrafeMapValue`) 0.0 1.0 (.x (100.0 50.0 30.0)) _y) (`KismetMathLibrary.MapRangeClamped` (`local.StrafeMapValue`) 1.0 2.0 _y (.z (100.0 50.0 30.0))) (< (`local.StrafeMapValue`) 1.0))))

(fn `CalculateGroundFriction`
  (returns (`Return Value` :type "Float (double-precision)"))
  (return (select `/Game/Nahoo_Locomotion_System/Data/Struct/Enum-Gait` (`self.m-gait`) :`NewEnumerator0` 5.0 :`NewEnumerator1` 5.0 :`NewEnumerator2` (`KismetMathLibrary.MapRangeClamped` (`KismetMathLibrary.VSizeXYSquared` (`MovementComponent.Velocity` (`self.CharacterMovement`))) 0.0 250000.0 5.0 3.0))))

(fn `CalculateMaxAcceleration`
  (returns (ReturnValue :type "Float (double-precision)"))
  (return (select `/Game/Nahoo_Locomotion_System/Data/Struct/Enum-Gait` (`self.m-gait`) :`NewEnumerator0` 800.0 :`NewEnumerator1` 800.0 :`NewEnumerator2` (`KismetMathLibrary.MapRangeClamped` (`KismetMathLibrary.VSizeXYSquared` (`MovementComponent.Velocity` (`self.CharacterMovement`))) 90000.0 490000.0 800.0 300.0))))

(fn `CalculateMaxSpeed`
  (returns (`Return Value` :type "Float (double-precision)"))
  (locals (StraftMapValue :type "Float (double-precision)"))
  (bind (_returnvalue_x _returnvalue_y _returnvalue_z) (`KismetMathLibrary.BreakVector` (select `/Game/Nahoo_Locomotion_System/Data/Struct/Enum-Gait` (`self.m-gait`) :`NewEnumerator0` (`self.m-walkSpeed`) :`NewEnumerator1` (`self.m-runSpeed`) :`NewEnumerator2` (`self.m-sprintSpeed`))))
  (set `local.StraftMapValue` (select `bool` (`CharacterMovementComponent.bUseControllerDesiredRotation` (`self.CharacterMovement`)) :`true` (`CurveFloat.GetFloatValue` (`self.m-strafeMap`) (`KismetMathLibrary.Abs` (`KismetAnimationLibrary.CalculateDirection` (`MovementComponent.Velocity` (`self.CharacterMovement`)) (`self.K2_GetActorRotation`))))))
  (return (`KismetMathLibrary.SelectFloat` (`KismetMathLibrary.MapRangeClamped` (`local.StraftMapValue`) 0.0 1.0 _returnvalue_x _returnvalue_y) (`KismetMathLibrary.MapRangeClamped` (`local.StraftMapValue`) 1.0 2.0 _returnvalue_y _returnvalue_z) (< (`local.StraftMapValue`) 1.0))))

(fn `CanSprint`
  (returns (`Return Value` :type Boolean))
  (bind (_returnvalue_roll _returnvalue_pitch _returnvalue_yaw) (`KismetMathLibrary.BreakRotator` (`KismetMathLibrary.NormalizedDeltaRotator` (`self.K2_GetActorRotation`) (`KismetMathLibrary.MakeRotFromX` (`CharacterMovementComponent.GetCurrentAcceleration` (`self.CharacterMovement`))))))
  (return (and (`.WanttoSprint_7_1D0B938A4EB6C1FD7D7DCFBCDCED247E` (break `/Game/Nahoo_Locomotion_System/Data/Struct/S-InputState` (`self.m-inputState`))) (select `bool` (`CharacterMovementComponent.bOrientRotationToMovement` (`self.CharacterMovement`)) :`false` (< (`KismetMathLibrary.Abs` _returnvalue_yaw) 50.0) :`true` true))))

(fn `GetDesiredGait`
  (returns (Gait :type "/Game/Nahoo_Locomotion_System/Data/Struct/Enum-Gait Enum"))
  (if (`self.CanSprint`)
    (return "NewEnumerator2")
    (elif (`.WanttoWalk_6_6818E2C94269A81E3DF7B3BEBC39940F` (break `/Game/Nahoo_Locomotion_System/Data/Struct/S-InputState` (`self.m-inputState`)))
      (return "NewEnumerator0")
      (else
        (return "NewEnumerator1")))))

(fn `Nahoo_Crouch`
  (if (not (`NavMovementComponent.IsFalling` (`self.CharacterMovement`)))
    (if (`self.bIsCrouched`)
      (`self.UnCrouch`)
      (else
        (`self.Crouch`)))))

(fn `Nahoo_Jump`
  (params (`Action Value` :type Boolean))
  (`|ExecutionSequence`
    (:`then_0`
      (if (`self.bIsCrouched`)
        (`self.UnCrouch`)))
    (:`then_1`
      (if (`local.Action Value`)
        (`self.Jump`)
        (else
          (`self.StopJumping`))))))

(fn `Nahoo_Look`
  (params (`Y-axis` :type "Float (double-precision)") (`Z-axis` :type "Float (double-precision)"))
  (`|ExecutionSequence`
    (:`then_0`
      (`self.AddControllerPitchInput` (`local.Y-axis`)))
    (:`then_1`
      (`self.AddControllerYawInput` (`local.Z-axis`)))))

(fn `Nahoo_Move`
  (params (`X-axis` :type "Float (double-precision)") (`Y-axis` :type "Float (double-precision)"))
  (bind (_returnvalue_roll _returnvalue_pitch _returnvalue_yaw) (`KismetMathLibrary.BreakRotator` (`self.GetControlRotation`)))
  (bind (_returnvalue_roll_2 _returnvalue_pitch_2 _returnvalue_yaw_2) (`KismetMathLibrary.BreakRotator` (`self.GetControlRotation`)))
  (`|ExecutionSequence`
    (:`then_0`
      (`self.AddMovementInput` (`KismetMathLibrary.GetRightVector` (`KismetMathLibrary.MakeRotator` _returnvalue_roll_2 0.0 _returnvalue_yaw_2)) (`local.Y-axis`)))
    (:`then_1`
      (`self.AddMovementInput` (`KismetMathLibrary.GetForwardVector` (`KismetMathLibrary.MakeRotator` 0.0 0.0 _returnvalue_yaw)) (`local.X-axis`)))))

(fn `Nahoo_WalkToggle`
  (bind ((`WanttoWalk_6_6818E2C94269A81E3DF7B3BEBC39940F` _wanttowalk) (`WanttoSprint_7_1D0B938A4EB6C1FD7D7DCFBCDCED247E` _wanttosprint)) (break `/Game/Nahoo_Locomotion_System/Data/Struct/S-InputState` (`self.m-inputState`)))
  (if (not _wanttosprint)
    (setmembers `/Game/Nahoo_Locomotion_System/Data/Struct/S-InputState` :`StructRef` (`self.m-inputState`) :`Want to Walk` (not _wanttowalk))))

(fn `UpdateMovement`
  (`|ExecutionSequence`
    (:`then_0`
      (set `self.m-gait` (`self.GetDesiredGait`)))
    (:`then_1`
      (set `CharacterMovementComponent.MaxAcceleration` (`self.CalculateMaxAcceleration`) (`self.CharacterMovement`))
      (set `CharacterMovementComponent.BrakingDecelerationWalking` (`self.CalculateBrakingDeceleration`) (`self.CharacterMovement`))
      (set `CharacterMovementComponent.GroundFriction` (`self.CalculateGroundFriction`) (`self.CharacterMovement`)))
    (:`then_2`
      (set `CharacterMovementComponent.MaxWalkSpeed` (`self.CalculateMaxSpeed`) (`self.CharacterMovement`))
      (set `CharacterMovementComponent.MaxWalkSpeedCrouched` (`self.CalculateCrouchMaxSpeed`) (`self.CharacterMovement`)))))

(fn `UpdateRotation`
  (bind _charactermovement (`self.CharacterMovement`))
  (bind _charactermovement_2 (`self.CharacterMovement`))
  (bind ((`WanttoStrafe_4_485767C946B920090F31B3BADF768C4E` _wanttostrafe) (`WanttoAim_5_1227E4FE4F183B761D11A9B297EEADB2` _wanttoaim)) (break `/Game/Nahoo_Locomotion_System/Data/Struct/S-InputState` (`self.m-inputState`)))
  (`|ExecutionSequence`
    (:`then_0`
      (if (or _wanttostrafe _wanttoaim)
        (set `CharacterMovementComponent.bUseControllerDesiredRotation` true _charactermovement_2)
        (set `CharacterMovementComponent.bOrientRotationToMovement` false _charactermovement_2)
        (else
          (set `CharacterMovementComponent.bUseControllerDesiredRotation` false _charactermovement)
          (set `CharacterMovementComponent.bOrientRotationToMovement` true _charactermovement))))
    (:`then_1`
      (if (`NavMovementComponent.IsFalling` (`self.CharacterMovement`))
        (set `CharacterMovementComponent.RotationRate` (struct :`Yaw` 200.0) (`self.CharacterMovement`))
        (else
          (set `CharacterMovementComponent.RotationRate` (struct :`Yaw` -1.0) (`self.CharacterMovement`)))))))

(fn `UserConstructionScript`)