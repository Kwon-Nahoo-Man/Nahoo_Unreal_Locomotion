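; Anim notify state meant to trigger early transitions in ABP-Nahoo_Base, apparently left unfinished or disabled.
; Each tick outside blend-out, it casts the anim instance and sets Transition from TransitionCondition: true for Always, false for Gait Not Equal.
; The TransitionDestination switch has empty outputs, with the loop and re-transition flag setters disconnected.
; The gait comparison and descriptive notify-name builder are also unwired, so GetNotifyName returns an empty string.
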(fn `GetNotifyName`
  (returns (ReturnValue :type String))
  (return ""))

(fn `Received_NotifyTick`
  (params (MeshComp :type "SkeletalMeshComponent Object Reference") (Animation :type "AnimSequenceBase Object Reference") (FrameDeltaTime :type "Float (single-precision)") (EventReference :type "AnimNotifyEventReference Structure (by ref)"))
  (returns (ReturnValue :type Boolean))
  (locals (Character :type "Object Object Reference") (Transition :type Boolean))
  (bind _asabp_nahoo_base (cast `/Game/Nahoo_Locomotion_System/Character/Mannequin/AnimBlueprint/ABP-Nahoo_Base` (`SkeletalMeshComponent.GetAnimInstance` MeshComp)))
  (set `local.Character` _asabp_nahoo_base)
  (if (not (`AnimNotifyLibrary.IsBlendingOut` (`local.EventReference`)))
    (`|ExecutionSequence`
      (:`then_0`
        (switch `/Game/Blueprints/AnimNotifies/E_EarlyTransition_Condition` (`self.TransitionCondition`)
          (:`NewEnumerator1`
            (set `local.Transition` true))
          (:`NewEnumerator0`
            (set `local.Transition` false))))
      (:`then_1`
        (if (`local.Transition`)
          (switch `/Game/Blueprints/AnimNotifies/E_EarlyTransition_Destination` (`self.TransitionDestination`)))))))